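; Door furniture Blueprint that toggles open and closed, with a sound, through the DrawerInteract event.
; A FlipFlop plays the OpenCloseDoor timeline forward from start or in reverse from end on alternate calls.
; Timeline tracks drive the passed component's yaw swing and the pitch turn of both handles.
; The component's roll and pitch are fed from its relative location Y and Z, not its rotation.
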(event `self.DrawerInteract`
  (params (Component :type "PrimitiveComponent Object Reference"))
  (bind (_relativelocation_x _relativelocation_y _relativelocation_z) (`KismetMathLibrary.BreakVector` (`SceneComponent.RelativeLocation` Component)))
  (`/Engine/EditorBlueprintResources/StandardMacros.FlipFlop`
    (:`A`
      (`GameplayStatics.PlaySound2D` "/Game/Audio/Door/OpenDoor.OpenDoor" 1.0 1.0 0.0 null null)
      (bind (_direction _openclose _doorhandle) (`Timeline|OpenCloseDoor` :!via `PlayFromStart` :!label _label)
        (:`Update`
          (`SceneComponent.K2_SetRelativeRotation` Component (`KismetMathLibrary.MakeRotator` _relativelocation_y _relativelocation_z (`KismetMathLibrary.Lerp` 0.0 80.0 _openclose)) false false)
          (`SceneComponent.K2_SetRelativeRotation` (`self.Handle`) (`KismetMathLibrary.MakeRotator` 0.0 (`KismetMathLibrary.Lerp` 0.0 40.0 _doorhandle) 89.0) false false)
          (`SceneComponent.K2_SetRelativeRotation` (`self.Handle1`) (`KismetMathLibrary.MakeRotator` 0.0 (`KismetMathLibrary.Lerp` 0.0 40.0 _doorhandle) 89.0) false false))))
    (:`B`
      (`GameplayStatics.PlaySound2D` "/Game/Audio/Door/CloseDoor.CloseDoor" 1.0 1.0 0.0 null null)
      (goto _label :!via `ReverseFromEnd`))))

(fn `UserConstructionScript`)