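; Fridge (Kulkas) furniture Blueprint whose DrawerInteract event swings a given component open or closed with a sound.
; The component's current yaw picks the direction, playing the OpenCloseDrawer timeline forward to close or in reverse to open.
; The timeline lerps relative yaw between -90 and 0 degrees, preserving roll and pitch.
; The OpenDrawer branch has no effect, and the node setting that flag true is never reached.
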(event `self.DrawerInteract`
  (params (Component :type "PrimitiveComponent Object Reference"))
  (bind (_relativerotation_roll _relativerotation_pitch _relativerotation_yaw) (`KismetMathLibrary.BreakRotator` (`SceneComponent.RelativeRotation` Component)))
  (if (`self.OpenDrawer`)
    _
    (else
      _))
  (if (not (> _relativerotation_yaw -90.0))
    (`GameplayStatics.PlaySound2D` "/Game/Audio/Drawer/CloseCuboard.CloseCuboard" 1.0 1.0 0.0 null null)
    (bind (_direction _openclose) (`Timeline|OpenCloseDrawer` :!via `PlayFromStart` :!label _label)
      (:`Update`
        (`SceneComponent.K2_SetRelativeRotation` Component (`KismetMathLibrary.MakeRotator` _relativerotation_roll _relativerotation_pitch (`KismetMathLibrary.Lerp` -90.0 0.0 _openclose)) false false))
      (:`Finished`
        (set `self.OpenDrawer` false)))
    (else
      (`GameplayStatics.PlaySound2D` "/Game/Audio/Drawer/OpenCuboard.OpenCuboard" 1.0 1.0 0.0 null null)
      (goto _label :!via `ReverseFromEnd`))))

(fn `UserConstructionScript`)