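; Oil lamp furniture Blueprint that lights up once when its InteractSystem event is triggered.
; The OpenGlass timeline raises the glass chimney, then reverses after a delay to lower it, with timed open, match-strike and close sounds.
; The same timeline's update, after a short delay, drives the point light intensity and unhides the candle flame.
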(event `/Game/ThirdPerson/Blueprints/System/HororInterface.InteractSystem`
  (`/Engine/EditorBlueprintResources/StandardMacros.DoOnce` false
    (:`Completed`
      (`|ExecutionSequence`
        (:`then_0`
          (`GameplayStatics.PlaySound2D` "/Game/Audio/Flashlight/BukaKaca.BukaKaca" 1.0 1.0 0.0 null null)
          (`|ExecutionSequence`
            (:`then_0`
              (bind (_direction _open _light) (`Timeline|OpenGlass` :!via `PlayFromStart` :!label _label)
                (:`Update`
                  (`SceneComponent.K2_SetRelativeLocation` (`self.KacaLampu`) (`KismetMathLibrary.MakeVector` -0.160466 3.281404 (`KismetMathLibrary.Lerp` 37.994977 75.518644 _open)) false false)
                  (`KismetSystemLibrary.Delay` 1.0)
                  (`LightComponent.SetIntensity` (`self.PointLight`) (+ _light 1000.0))
                  (`SceneComponent.SetHiddenInGame` (`self.0_CandleFire_pt`) false false))))
            (:`then_1`
              (`KismetSystemLibrary.Delay` 1.0)
              (`GameplayStatics.PlaySound2D` "/Game/Audio/Flashlight/Korek.Korek" 1.0 1.0 0.0 null null)
              (`KismetSystemLibrary.Delay` 1.8)
              (`GameplayStatics.PlaySound2D` "/Game/Audio/Flashlight/TutupKaca.TutupKaca" 1.0 1.0 0.0 null null))))
        (:`then_1`
          (`KismetSystemLibrary.Delay` 2.3)
          (goto _label :!via `ReverseFromEnd`))))))

(fn `UserConstructionScript`)