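; BP_Laci2 is a furniture Blueprint whose drawers slide open and closed on interaction.
; DrawerInteract takes the drawer component and reads its relative X position to decide whether to open or close it.
; One shared timeline, played forward or in reverse, lerps that X position, with a 2D sound for each direction.
; The OpenDrawer flag is effectively inert, as the node setting it true never runs.
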(event `self.DrawerInteract`
  (params (Component :type "PrimitiveComponent Object Reference"))
  (bind (_relativelocation_x _relativelocation_y _relativelocation_z) (`KismetMathLibrary.BreakVector` (`SceneComponent.RelativeLocation` Component)))
  (if (`self.OpenDrawer`)
    _
    (else
      _))
  (if (not (> _relativelocation_x 51.991769))
    (`GameplayStatics.PlaySound2D` "/Game/Audio/Drawer/OpenDrawer.OpenDrawer" 1.0 1.0 0.0 null null)
    (bind (_direction _openclose) (`Timeline|OpenCloseDrawer` :!via `PlayFromStart` :!label _label)
      (:`Update`
        (`SceneComponent.K2_SetRelativeLocation` Component (`KismetMathLibrary.MakeVector` (`KismetMathLibrary.Lerp` 24.22135 52.991769 _openclose) _relativelocation_y _relativelocation_z) false false))
      (:`Finished`
        (set `self.OpenDrawer` false)))
    (else
      (`GameplayStatics.PlaySound2D` "/Game/Audio/Drawer/CloseDarawer.CloseDarawer" 1.0 1.0 0.0 null null)
      (goto _label :!via `ReverseFromEnd`))))

(fn `UserConstructionScript`)