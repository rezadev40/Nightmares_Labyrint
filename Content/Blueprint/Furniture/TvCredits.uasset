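; TvCredits is an interactable TV furniture actor that toggles the player's view between the TV and the third-person character.
; InteractSystem drives a FlipFlop: the first use switches the view target to the TvCredits actor and hides the character, the next restores both.
; Both view targets are found by class with GetActorOfClass, so the TV targets the first TvCredits found rather than explicitly itself.
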(event `/Game/ThirdPerson/Blueprints/System/HororInterface.InteractSystem`
  (`/Engine/EditorBlueprintResources/StandardMacros.FlipFlop`
    (:`A`
      (bind _returnvalue (`GameplayStatics.GetActorOfClass` "TvCredits_C"))
      (`PlayerController.SetViewTargetWithBlend` (`GameplayStatics.GetPlayerController` 0) _returnvalue 0.0 "VTBlend_Linear" 1.0 false)
      (bind _asbp_third_person_character (cast `/Game/ThirdPerson/Blueprints/BP_ThirdPersonCharacter` (`GameplayStatics.GetPlayerCharacter` 0)))
      (`SceneComponent.SetHiddenInGame` (`/Game/ThirdPerson/Blueprints/BP_ThirdPersonCharacter.Character` _asbp_third_person_character) true false))
    (:`B`
      (bind _returnvalue_2 (`GameplayStatics.GetActorOfClass` "/Game/ThirdPerson/Blueprints/BP_ThirdPersonCharacter.BP_ThirdPersonCharacter_C"))
      (`PlayerController.SetViewTargetWithBlend` (`GameplayStatics.GetPlayerController` 0) _returnvalue_2 0.0 "VTBlend_Linear" 1.0 false)
      (bind _asbp_third_person_character_2 (cast `/Game/ThirdPerson/Blueprints/BP_ThirdPersonCharacter` (`GameplayStatics.GetPlayerCharacter` 0)))
      (`SceneComponent.SetHiddenInGame` (`/Game/ThirdPerson/Blueprints/BP_ThirdPersonCharacter.Character` _asbp_third_person_character_2) false false))))

(fn `UserConstructionScript`)