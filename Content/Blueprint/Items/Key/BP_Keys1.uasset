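; Key actor that the player can inspect up close through a toggled interaction.
; InteractSystem flip-flops behind a DoOnce: timelines lerp the key to the character's InspectItems transform and back to the transform cached at BeginPlay.
; Inspecting shows the Key1 name/description widget, removes ButtonMain and locks movement and look; returning reverses the lock and removes Key1.
; RotateUp and Tick share a roll-rotation branch gated by Inspect, which this graph never sets.
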(event `self.ReceiveTick`
  (params (DeltaSeconds :type "Float (single-precision)"))
  (if (`self.Inspect`) :!label _label
    (`SceneComponent.K2_AddLocalRotation` (`self.Key`) (`KismetMathLibrary.MakeRotator` (* (stale `RotateUp` A) 1.0)) false false)))

(event `RotateUp`
  (params (A :type "Float (double-precision)"))
  (goto _label))

(event `self.ReceiveBeginPlay`
  (bind _key (`self.Key`))
  (bind _output_get (set `self.Rotation` (`SceneComponent.K2_GetComponentLocation` _key)))
  (bind _output_get_2 (set `self.Locations` (`SceneComponent.K2_GetComponentRotation` _key))))

(event `self.InteractSystem`
  (`/Engine/EditorBlueprintResources/StandardMacros.DoOnce` false :!label _label_2
    (:`Completed`
      (`/Engine/EditorBlueprintResources/StandardMacros.FlipFlop`
        (:`A`
          (bind _asbp_third_person_character (cast `/Game/ThirdPerson/Blueprints/BP_ThirdPersonCharacter` (`GameplayStatics.GetPlayerCharacter` 0)))
          (bind _returnvalue (`|CreateWidget` "/Game/Blueprint/UI/KeyInspect/Key1.Key1_C" null (`self.Nama Items`) (`self.Deskripsi Items`)))
          (`UserWidget.AddToViewport` _returnvalue 0)
          (`CharacterMovementComponent.DisableMovement` (`Character.CharacterMovement` (`GameplayStatics.GetPlayerCharacter` 0)))
          (`Controller.SetIgnoreLookInput` (`GameplayStatics.GetPlayerController` 0) true)
          (bind (_direction _inspect) (`Timeline|Timeline` :!via `PlayFromStart`)
            (:`Update`
              (bind (_returnvalue_location _returnvalue_rotation) (`KismetMathLibrary.BreakTransform` (`SceneComponent.K2_GetComponentToWorld` (`/Game/ThirdPerson/Blueprints/BP_ThirdPersonCharacter.InspectItems` _asbp_third_person_character))))
              (`SceneComponent.K2_SetWorldTransform` (`self.Key`) (`KismetMathLibrary.MakeTransform` (`KismetMathLibrary.VLerp` (stale `self.ReceiveBeginPlay` _output_get) _returnvalue_location _inspect) (`KismetMathLibrary.RLerp` (stale `self.ReceiveBeginPlay` _output_get_2) _returnvalue_rotation _inspect)) false false)
              (bind _foundwidgets (`WidgetBlueprintLibrary.GetAllWidgetsOfClass` "/Game/Blueprint/UI/ButtonMain.ButtonMain_C"))
              (`Widget.RemoveFromParent` _foundwidgets)
              (goto _label_2 :!via `Reset`))))
        (:`B`
          (bind _asbp_third_person_character_2 (cast `/Game/ThirdPerson/Blueprints/BP_ThirdPersonCharacter` (`GameplayStatics.GetPlayerCharacter` 0)))
          (`CharacterMovementComponent.SetMovementMode` (`Character.CharacterMovement` _asbp_third_person_character_2) "MOVE_Walking" 0)
          (`Controller.ResetIgnoreLookInput` (`GameplayStatics.GetPlayerController` 0))
          (bind (_direction_2 _inspect_2) (`Timeline|Timeline_0` :!via `PlayFromStart`)
            (:`Update`
              (`SceneComponent.K2_SetWorldTransform` (`self.Key`) (`KismetMathLibrary.MakeTransform` (`KismetMathLibrary.VLerp` _returnvalue_location (stale `self.ReceiveBeginPlay` _output_get) _inspect_2) (`KismetMathLibrary.RLerp` _returnvalue_rotation (stale `self.ReceiveBeginPlay` _output_get_2) _inspect_2)) false false)
              (bind _foundwidgets_2 (`WidgetBlueprintLibrary.GetAllWidgetsOfClass` "/Game/Blueprint/UI/KeyInspect/Key1.Key1_C"))
              (`Widget.RemoveFromParent` _foundwidgets_2))
            (:`Finished`
              (goto _label_2 :!via `Reset`))))))))

(fn `UserConstructionScript`)