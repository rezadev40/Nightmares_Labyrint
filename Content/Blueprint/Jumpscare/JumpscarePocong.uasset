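; A pocong jumpscare trigger actor that fires when something overlaps its Box, playing a 2D scare sound for any actor.
; For BP_ThirdPersonCharacter, it calls the character's Jumpscare, reveals the looping animated Copong mesh and turns on a RectLight.
; After a delay it switches the light off and destroys itself.
; A parallel Sequence branch damages the player after a shorter delay, before the actor is destroyed.
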(event `self.Box.OnComponentBeginOverlap`
  (params (OverlappedComponent :type "PrimitiveComponent Object Reference") (OtherActor :type "Actor Object Reference") (OtherComp :type "PrimitiveComponent Object Reference") (OtherBodyIndex :type Integer) (bFromSweep :type Boolean) (SweepResult :type "HitResult Structure (by ref)"))
  (bind _copong (`self.Copong`))
  (bind _rectlight (`self.RectLight`))
  (`GameplayStatics.PlaySound2D` "/Game/Audio/Jumpsacre1.Jumpsacre1" 1.0 1.0 0.0 null null)
  (bind _asbp_third_person_character (cast `/Game/ThirdPerson/Blueprints/BP_ThirdPersonCharacter` OtherActor))
  (`|ExecutionSequence`
    (:`then_0`
      (`/Game/ThirdPerson/Blueprints/BP_ThirdPersonCharacter.Jumpscare` _asbp_third_person_character)
      (`SceneComponent.SetHiddenInGame` _copong false false)
      (`SkeletalMeshComponent.PlayAnimation` _copong "/Game/Characters/Hantu/Ocong/Copong_Anim.Copong_Anim" true)
      (`LightComponent.SetIntensity` _rectlight 700.0)
      (`KismetSystemLibrary.Delay` 3.0)
      (`LightComponent.SetIntensity` _rectlight 0.0)
      (`self.K2_DestroyActor`))
    (:`then_1`
      (`KismetSystemLibrary.Delay` 2.0)
      (`/Game/ThirdPerson/Blueprints/BP_ThirdPersonCharacter.PlayerDamage` _asbp_third_person_character 20.0))))

(fn `UserConstructionScript`)